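; Battle royale game mode that triggers the death zone spawn shortly after play begins.
; BeginPlay prints a warning, waits five seconds, then calls a server spawn event that hands the work to RoyaleStormGameState.
; Its own SpawnDeathZone function, which places the zone at a random XY and announces the spawn, is called only from unconnected nodes.
; The authority switch has empty branches.
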(event Custom|Server_SpawnDeathZone
  (Default|SpawnDeathZone (.AsRoyale%20Storm%20Game%20State (Utilities|Casting|CastToRoyaleStormGameState (Game|GetGameState)))))

(event EventBeginPlay
  (Networking|SwitchHasAuthority
    (:Authority
      _)
    (:Remote
      _))
  (Development|PrintString "-- DEATHZONE SPAWNS IN 5 SECS --" true true "(R=1.000000,G=0.043376,B=0.000000,A=1.000000)" 5.0)
  (Utilities|FlowControl|Delay 5.0)
  (CallFunction|ServerSpawnDeathZone))

(fn ConstructionScript)

(fn SpawnDeathZone
  (bind _returnvalue (Math|Random|RandomFloatinRange -5e+03 5e+03))
  (bind _returnvalue_2 (Game|SpawnActorfromClass "/Game/Blueprints/DeathZoneBlueprints/DeathZoneBlueprint.DeathZoneBlueprint_C" (Math|Transform|MakeTransform (Math|Vector|MakeVector _returnvalue _returnvalue 0.0) "0, 0, 0" "1,1,1") "Undefined" 0 0))
  (Utilities|IsValid _returnvalue_2
    (:Is%20Valid
      (Default|CallOnDeathZoneSpawn))))