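; Base footprint type that defines the visual and audio response to a footfall through a supplied footprint component.
; OnFootFall has the component spawn a decal with either random or foot-aligned yaw, offset by 90 degrees.
; It also spawns tracking using a separate track material, body overlay texture and tracking sound.
; When their assets are valid, it plays a basic footprint sound with a speed-volume multiplier and spawns particles.
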(fn OnFootFall
  (params (FootLocation :type Vector) (FootRotation :type Rotator) (FootType :type ENEFootType%20Enum :default "NewEnumerator0") (FootprintComponent :type Footprint%20Component%20Object%20Reference))
  (bind _yaw (Math|Rotator|BreakRotator FootRotation))
  (Default|SpawnDecal FootprintComponent FootLocation (+ (select (Variables|BaseDecal|GetRandomRotation) (Math|Random|RandomFloatinRange -1.8e+02 1.8e+02) _yaw) 9e+01) (Variables|BaseDecal|GetDecalSize) (Variables|BaseDecal|GetFootPrintDecal) (Variables|BaseDecal|GetDecalLifespan) 0.0)
  ;[0 1 1 0.09804] Material Tracking
  (Default|SpawnTracking FootprintComponent FootLocation _yaw (Variables|BaseDecal|GetDecalSize) (Variables|BaseDecal|GetDecalLifespan) (Variables|Tracking|GetBodyTrackMaterial) (Variables|Tracking|GetFootTrackDecal) (Variables|Tracking|GetTrackingFootprintSound))
  (bind _basicfootprintsound (Variables|Audio|GetBasicFootprintSound)
    (:then
      (Default|PlayBasicFootprintSound FootprintComponent FootLocation _basicfootprintsound (Variables|Audio|GetSpeedVolumeMultiplier)))
    (:else
      _))
  (bind _particleeffect (Variables|Particle|GetParticleEffect)
    (:then
      (Default|SpawnParticles FootprintComponent FootLocation FootRotation _particleeffect))
    (:else)))